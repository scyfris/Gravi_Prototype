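; GraviPlayerController is a player controller that sets up pointer input and the game's camera view.
; On BeginPlay it enables click events on player controller 0 and turns on mouse-over events.
; It then makes the first MyCamera actor found in the level that controller's view target.
; Its actor click and touch-end handlers only print placeholder debug strings.
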(event EventBeginPlay
  (Variables|/Script/Engine.PlayerController|SetbEnableClickEvents (Game|GetPlayerController 0) true)
  (Variables|Default|SetbEnableMouseOverEvents true)
  (bind _outactors (Actor|GetAllActorsOfClass "/Game/Blueprints/MyCamera.MyCamera_C"))
  (Game|Player|SetViewTargetwithBlend (Game|GetPlayerController 0) (Utilities|Array|Get(acopy) _outactors) 0.0 "VTBlend_Linear" 0.0 false))

(event EventTick
  (params (DeltaSeconds :type Float%20%28single-precision%29)))

(event MouseInput|EventActorOnClicked
  (params (ButtonPressed :type Key%20Structure :default "AnyKey"))
  (Development|PrintString "Hello"))

(event EventActorOnInputTouchEnd
  (params (FingerIndex :type ETouchIndex%20Enum :default "Touch1"))
  (Development|PrintString "RAR"))

(fn ConstructionScript)