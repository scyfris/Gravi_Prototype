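; ExpandingRing2 is an effect actor that displays expanding rings through a parameterized material on its Cube component.
; The construction script creates a dynamic material instance from the Cube's first material slot, applies it, and stores it.
; AssignMaterialParams then pushes the zoom, wave count, wave width, time scale and ring color variables into that instance.
; It has no runtime logic, so any animation is left to the material.
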(event EventBeginPlay)

(event Collision|EventActorBeginOverlap
  (params (OtherActor :type Actor%20Object%20Reference)))

(event EventTick
  (params (DeltaSeconds :type Float%20%28single-precision%29)))

(fn ConstructionScript
  (bind _cube (Variables|Default|GetCube))
  (bind _returnvalue (Rendering|Material|CreateDynamicMaterialInstance _cube 0 (Rendering|Material|GetMaterial _cube 0) :!class /Script/Engine.PrimitiveComponent))
  (Rendering|Material|SetMaterial (Variables|Default|GetCube) 0 _returnvalue)
  (Variables|Default|SetMaterialInstance _returnvalue)
  (CallFunction|AssignMaterialParams))

(fn AssignMaterialParams
  (bind _materialinstance (Variables|Default|GetMaterialInstance))
  (Rendering|Material|SetScalarParameterValue _materialinstance "ZoomFactor" (Variables|RingProperties|GetZoomFactor) :!class /Script/Engine.MaterialInstanceDynamic)
  (Rendering|Material|SetScalarParameterValue _materialinstance "Waves" (Variables|RingProperties|GetWaves) :!class /Script/Engine.MaterialInstanceDynamic)
  (Rendering|Material|SetScalarParameterValue _materialinstance "TimeScale" (Variables|RingProperties|GetTimeScale) :!class /Script/Engine.MaterialInstanceDynamic)
  (Rendering|Material|SetScalarParameterValue _materialinstance "WaveWidth" (Variables|RingProperties|GetWaveWidth) :!class /Script/Engine.MaterialInstanceDynamic)
  (Rendering|Material|SetVectorParameterValue _materialinstance "RingColor" (Variables|RingProperties|GetRingColor) :!class /Script/Engine.MaterialInstanceDynamic))