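; Player actor for a gravity-based 2D tilemap game, rolling along the axis perpendicular to gravity from axis or touch-drag input.
; Tick feeds gravity and input into PhysicalRayboxBP's custom raycast physics, then applies the returned displacement and spin.
; Its collision dispatcher triggers death on "bad" tiles and level loading on LevelGoal hits.
; Also handles level rotation and pausing; an older in-Blueprint physics implementation remains, disconnected from execution.
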(event Custom|GraviTouchPressed
  ;[1 1 1] Player's touch events
  (Variables|Default|SetisPlayerDragging true))

(event Custom|PlayerCollision
  (params (Collision%20Ray%20Hit :type Hit%20Result%20Structure))
  ;[1 1 1] Bind collision events with raybox bp
  (CallFunction|HandleHitwithSpecialObjects Collision%20Ray%20Hit))

(event Custom|GraviTouchReleased
  ;[1 1 1] Player's touch events
  (Variables|Default|SetisPlayerDragging false))

(event Custom|PlayerDeath
  (bind _returnvalue (Game|GetPlayerController 0))
  ;[1 1 1] Player death
  (Utilities|IsValid (Variables|Default|GetDeath%20Menu%20Reference)
    (:Is%20Valid
      _)
    (:Is%20Not%20Valid
      (bind _returnvalue_2 (UserInterface|CreateWidget "/Game/Blueprints/Menus/DeathMenu.DeathMenu_C"))
      (Variables|Default|SetDeath%20Menu%20Reference _returnvalue_2)))
  (Input|SetInputModeUIOnly _returnvalue (Variables|Default|GetDeath%20Menu%20Reference) "DoNotLock")
  (Variables|/Script/Engine.PlayerController|SetbShowMouseCursor _returnvalue true)
  (UserInterface|Viewport|AddtoViewport (Variables|Default|GetDeath%20Menu%20Reference) 0)
  (Game|SetGamePaused true))

(event Custom|PlayerLevelGoal
  (params (NewParam :type Level%20Goal%20Object%20Reference))
  ;[1 1 1] Player hitting level goal
  (Game|OpenLevel(byName) (Utilities|String|StringToName (Variables|/Game/Blueprints/LevelObjects/LevelGoal.LevelGoal_C|GetNextLevelName NewParam))))

(event Custom|TileCollisionEvent
  (params (tileInfo :type Paper%20Tile%20Info%20Structure) (tileMapCompRef :type Paper%20Tile%20Map%20Component%20Object%20Reference))
  ;[1 1 1] Tile hit event
  (if (Utilities|Enum|Equal(Enum) (Utilities|String|ToString(Name) (Class|TileMapBlueprintLibrary|GetTileUserData tileInfo)) "bad")
    ;[1 1 1] Player hit a death tile
    (CallFunction|PlayerDeath)))

(event Custom|GraviTouchMoved
  (params (ScreenPosition :type Vector))
  ;[1 1 1] Player's touch events
  (Variables|Default|SetdraggingTowards (.WorldPosition (Class|GameplayStatics|DeprojectScreentoWorld (Game|GetPlayerController 0) (Math|Conversions|ToVector2D(Vector) ScreenPosition))))
  (CallFunction|HandleTouchInput))

(event EventBeginPlay
  (bind _returnvalue (Game|GetPlayerController 0))
  (Input|SetInputModeGameOnly (Game|GetPlayerController 0))
  (Variables|/Script/Engine.PlayerController|SetbShowMouseCursor _returnvalue true)
  (Variables|/Script/Engine.PlayerController|SetbEnableClickEvents _returnvalue true)
  (Variables|/Script/Engine.PlayerController|SetbEnableMouseOverEvents _returnvalue true)
  (Input|EnableInput _returnvalue)
  (EventDispatchers|BindEventtoCollisionEventDispatcher (Variables|Default|GetPhysicalRayboxBP) (delegate Custom|PlayerCollision)))

(event Collision|EventActorBeginOverlap
  (params (OtherActor :type Actor%20Object%20Reference))
  ;[1 1 1] Events
)

(event EventTick
  (params (DeltaSeconds :type Float%20%28single-precision%29))
  (bind _gravityvector (Variables|Physics|GetGravityVector))
  (bind _physicalrayboxbp (Variables|Default|GetPhysicalRayboxBP))
  (bind _returnvalue (Class|GraviUtilities|GetPerpDirectionCounterClockwise3D _gravityvector))
  (bind _returnvalue_2 (Class|GraviUtilities|Get2DVector _returnvalue))
  ;[1 1 1] Events
  (Utilities|FlowControl|Sequence
    (:then_0
      ;[1 1 1] Move with mouse drags
      (CallFunction|HandleTouchInput))
    (:then_1
      (Variables|/Game/Blueprints/Components/PhysicalRayboxBP.PhysicalRayboxBP_C|SetRayBoxRayLengths _physicalrayboxbp (Variables|RayBoxInfo|GetRayBoxRayLength))
      (Variables|/Game/Blueprints/Components/PhysicalRayboxBP.PhysicalRayboxBP_C|SetRayBoxRayOffsets _physicalrayboxbp (Variables|RayBoxInfo|GetRayBoxOffsets))
      (Variables|/Game/Blueprints/Components/PhysicalRayboxBP.PhysicalRayboxBP_C|SetRayBoxNumRaysPerSide _physicalrayboxbp (Variables|RayBoxInfo|GetRayBoxNumPerSide))
      (Variables|/Game/Blueprints/Components/PhysicalRayboxBP.PhysicalRayboxBP_C|SetRayBoxGeo _physicalrayboxbp (Variables|Default|GetRayBox_Geo))
      (Variables|/Game/Blueprints/Components/PhysicalRayboxBP.PhysicalRayboxBP_C|SetGravity _physicalrayboxbp (Class|GraviUtilities|Get2DVector (Variables|Physics|GetGravityVector)))
      (Variables|/Game/Blueprints/Components/PhysicalRayboxBP.PhysicalRayboxBP_C|SetInputForcePerpDir _physicalrayboxbp (Variables|Input|GetRightAmount))
      (bind (_newvelocity _deltaposition) (Default|UpdatePhysics (Variables|Default|GetPhysicalRayboxBP) DeltaSeconds))
      (Development|PrintString (Utilities|String|ToString(Vector2d) _newvelocity))
      (Development|PrintString (Utilities|String|ToString(Vector2d) _deltaposition))
      (Transformation|AddActorWorldOffset (Class|GraviUtilities|Get3DVector _deltaposition 0.0))
      (if (> (Math|Vector2D|DotProduct(2D) (Class|GraviUtilities|GetVectorinDirection _deltaposition _returnvalue_2) _returnvalue_2) 0.0)
        (Transformation|AddWorldRotation (Variables|Default|Getplayer) (Math|Rotator|MakeRotator 0.0 (* (Math|Vector2D|Vector2DLength (Class|GraviUtilities|GetVectorinDirection _deltaposition _returnvalue_2)) -1.0) 0.0) false false)
        (elif (< (Math|Vector2D|DotProduct(2D) (Class|GraviUtilities|GetVectorinDirection _deltaposition _returnvalue_2) _returnvalue_2) 0.0)
          (Transformation|AddWorldRotation (Variables|Default|Getplayer) (Math|Rotator|MakeRotator 0.0 (Math|Vector2D|Vector2DLength (Class|GraviUtilities|GetVectorinDirection _deltaposition _returnvalue_2)) 0.0) false false))))
    (:then_2
      (Variables|input|SetShouldHaltFromTouchInput false))))

(event Input|ActionEvents|InputActionRotateRightDown
  (params (Key :type Key%20Structure :default "AnyKey"))
  ;[1 1 1] Events
  (:Pressed
    (Default|RotateLevel (Variables|ExternalRefs|GetLevelInfoRef) "NewEnumerator0")
    (Variables|Default|SetHealth (- (Variables|Default|GetHealth) 0.1))))

(event Input|AxisEvents|InputAxisMove
  (params (AxisValue :type Float%20%28single-precision%29))
  ;[1 1 1] Events
  ;[1 1 1] Handle Player Input
  (bind _canmove (CallFunction|CanMoveinDirection AxisValue))
  (if _canmove
    (Pawn|Input|AddMovementInput "1.000000, 0, 0" AxisValue false)
    (Variables|input|SetShouldHaltFromTouchInput false)))

(event Input|AxisEvents|InputAxisMove
  (params (AxisValue :type Float%20%28single-precision%29))
  ;[1 1 1] Events
  (Variables|Input|SetRightAmount (* AxisValue (Variables|Input|GetMoveSpeed))))

(event Input|KeyboardEvents|M
  (params (Key :type Key%20Structure :default "AnyKey"))
  (bind _returnvalue (Game|GetPlayerController 0))
  ;[1 1 1] Events
  ;;[1 1 1] Pause menu
  (:Pressed
    (Utilities|IsValid (Variables|Default|GetPause%20Menu%20Reference)
      (:Is%20Valid
        _)
      (:Is%20Not%20Valid
        (bind _returnvalue_2 (UserInterface|CreateWidget "/Game/Blueprints/Menus/PauseMenu.PauseMenu_C"))
        (Variables|Default|SetPause%20Menu%20Reference _returnvalue_2)))
    (Input|SetInputModeUIOnly _returnvalue (Variables|Default|GetPause%20Menu%20Reference) "DoNotLock")
    (Variables|/Script/Engine.PlayerController|SetbShowMouseCursor _returnvalue true)
    (UserInterface|Viewport|AddtoViewport (Variables|Default|GetPause%20Menu%20Reference) 0)
    (Game|SetGamePaused true)))

(event Input|TouchEvents|InputTouch
  (params (Location :type Vector) (FingerIndex :type ETouchIndex%20Enum))
  (:Released
    ;[1 1 1] Input touch
    (if (Variables|Default|GetisPlayerDragging)
      (Variables|Default|SetisPlayerDragging false)))
  (:Moved
    (if (Variables|Default|GetisPlayerDragging)
      _)))

(fn ConstructionScript)

(fn GetRayBoxCorners
  (params (CornerSelector :type BoxExtentSelector%20Enum))
  (bind _raybox_geo (Variables|Default|GetRayBox_Geo))
  (bind (_origin _boxextent) (Collision|GetComponentBounds _raybox_geo))
  (bind (_x _y _z) (Math|Vector|BreakVector _boxextent))
  (Utilities|FlowControl|Sequence
    (:then_0
      (switch Utilities|FlowControl|Switch|SwitchonBoxExtentSelector CornerSelector
        (:NewEnumerator0
          (LocalVariables|SetCornerMod 1.0))
        (:NewEnumerator1
          (LocalVariables|SetCornerMod -1.0))))
    (:then_1
      (return (+ _origin (Math|Vector|MakeVector (* _x (LocalVariables|GetCornerMod)) 0.0 (* _z -1.0)))))))

(fn CanMoveinDirection
  (params (Direction :type Float%20%28single-precision%29))
  ;[1 1 1] Never move on 0.0
  (if (!= Direction 0.0)
    ;[1 1 1] Can move, so set local variable StartOfRay
    (Utilities|FlowControl|Sequence
      (:then_0
        (if (> Direction 0.0)
          (LocalVariables|SetStartOfRay "0, 0, 0")
          (else
            (LocalVariables|SetStartOfRay "0, 0, 0"))))
      (:then_1
        ;[1 1 1] Use StartOfRay and check direction and determine if the object is about to fall off a ledge (can't move)
        (bind _outhit (Collision|LineTraceByChannel (LocalVariables|GetStartOfRay) (+ (LocalVariables|GetStartOfRay) (Math|Vector|MakeVector 0.0 0.0 (* (Variables|RayBoxInfo|GetRayBoxRayLength) -1.0))) "TraceTypeQuery1" false 0 "ForOneFrame"))
        (return (< (.Time (Collision|BreakHitResult _outhit)) 0.4))))
    (else
      (return false))))

(fn UpdatePhysics
  (params (DeltaTime :type Float%20%28single-precision%29) (rayCastResults :type Array%20of%20Ray%20Bundle%20Structures))
  (bind _gravityvector (Variables|Physics|GetGravityVector))
  (bind _returnvalue (CallFunction|GetPerpCounterClockwiseDir _gravityvector))
  (Utilities|FlowControl|Sequence
    (:then_0
      (LocalVariables|SetPerpGravDir _returnvalue)
      ;[1 1 1] Update Velocity
      (bind _output_get (Variables|Physics|SetVelocity (+ (* (* (Math|Vector|Normalize _returnvalue) (Variables|Input|GetRightAmount)) DeltaTime) (* (Variables|Physics|GetGravityVector) DeltaTime) (Variables|Physics|GetVelocity))))
      (if (< (Math|Vector|DotProduct _output_get (LocalVariables|GetPerpGravDir)) 0.0)
        (LocalVariables|SetisMovingLeft true)
        (elif (> (Math|Vector|DotProduct _output_get (LocalVariables|GetPerpGravDir)) 0.0)
          (LocalVariables|SetisMovingRight true))))
    (:then_1
      ;[1 1 1] get dV and dP in gravity direction
      (bind (_dposition _dvelocity _washit _collisionresultlist _collisionresultrayboxsideindex _collisionresultrayboxsideindexes) (CallFunction|GetDvDpinDirection (Variables|Physics|GetGravityVector) rayCastResults (Variables|Physics|GetVelocity) DeltaTime false (Variables|Physics|GetMaxFallSpeed)))
      (LocalVariables|SetDp (+ (LocalVariables|GetDp) _dposition))
      (LocalVariables|SetDv (+ (LocalVariables|GetDv) _dvelocity))
      (if _washit
        (for (_array_element _array_index) _collisionresultlist
          ;[1 1 1] Add our collision to the running collision results arrays.  This should be refactored into a separate array of custom structs or something
          (Utilities|Array|Add (LocalVariables|Getcollisionresults) _array_element)
          (Utilities|Array|Add (LocalVariables|Getcollisionresultsboxside) _collisionresultrayboxsideindex)
          (Utilities|Array|Add (LocalVariables|Getcollisionresultsboxsiderayindex) (Utilities|Array|Get(acopy) _collisionresultrayboxsideindexes _array_index)))
        ;[1 1 1] Determine if we are haning off left or right ledge, then prevent us from moving in that direction
        (if (<= (Utilities|Array|Length (LocalVariables|Getcollisionresults)) (/ 0 2))
          (if (== (Utilities|Array|Get(acopy) (LocalVariables|Getcollisionresultsboxsiderayindex)) 0)
            ;[1 1 1] Our left side is on the leddge, which means our right side is hanging off!
            (LocalVariables|SetcanMoveRight false)
            (else
              ;[1 1 1] Our right side is on the ledge, which means our left side is hanging off!
              (LocalVariables|SetcanMoveLeft false))))))
    (:then_2
      ;[1 1 1] Get dV dP in right/left direction
      (bind (_dposition_2 _dvelocity_2 _washit_2 _collisionresultlist_2) (CallFunction|GetDvDpinDirection (LocalVariables|GetPerpGravDir) rayCastResults (Variables|Physics|GetVelocity) DeltaTime (or (or (and (not (LocalVariables|GetcanMoveRight)) (LocalVariables|GetisMovingRight)) (and (not (LocalVariables|GetcanMoveLeft)) (LocalVariables|GetisMovingLeft))) (Variables|input|GetShouldHaltFromTouchInput)) (Variables|Physics|GetMaxInputSpeed)))
      (bind _output_get_2 (LocalVariables|Setdp_tang _dposition_2))
      (LocalVariables|SetDp (+ (LocalVariables|GetDp) _output_get_2))
      (bind _output_get_3 (LocalVariables|SetDv (+ (LocalVariables|GetDv) _dvelocity_2)))
      (if (> (Math|Vector|VectorLength _output_get_3) 0.0)
        (for _array_element_2 _collisionresultlist_2
          (Utilities|Array|Add (LocalVariables|Getcollisionresults) _array_element_2))))
    (:then_3
      ;[1 1 1] Update velocity and location after collisions
      (Variables|Physics|SetVelocity (+ (LocalVariables|GetDv) (Variables|Physics|GetVelocity)))
      (Transformation|AddActorWorldOffset (LocalVariables|GetDp))
      ;[1 1 1] Rotation of character
      (if (> (Math|Vector|DotProduct (LocalVariables|Getdp_tang) (LocalVariables|GetPerpGravDir)) 0.0)
        (Transformation|AddWorldRotation (Variables|Default|Getplayer) (Math|Rotator|MakeRotator 0.0 (* (Math|Vector|VectorLength (LocalVariables|Getdp_tang)) -1.0) 0.0) false false)
        (elif (< (Math|Vector|DotProduct (LocalVariables|Getdp_tang) (LocalVariables|GetPerpGravDir)) 0.0)
          (Transformation|AddWorldRotation (Variables|Default|Getplayer) (Math|Rotator|MakeRotator 0.0 (Math|Vector|VectorLength (LocalVariables|Getdp_tang)) 0.0) false false)))
      (return (LocalVariables|Getcollisionresults)))))

(fn CanFall)

(fn GetBoxDirIndexGivenVector
  (params (InVec :type Vector))
  (bind (_x _y _z) (Math|Vector|BreakVector InVec))
  (if (< _z 0.0)
    (return 0 1)
    (elif (> _x 0.0)
      (return 1 2)
      (elif (> _z 0.0)
        (return 2 3)
        (elif (< _x 0.0)
          (return 3 0)
          (else
            (Development|PrintString "Vector can't be 0,0,0 in Get Box Dir Index functions!!!!!" true true "(R=1.000000,G=0.000000,B=0.062970,A=1.000000)")
            (return 0 0)))))))

(fn HandleVelocityFunc
  (params (Velocity :type Vector) (DirVec :type Vector) (RayCastResults :type Array%20of%20Ray%20Bundle%20Structures))
  (bind _hitresultlistrayindexes (LocalVariables|GetHitResultListRayIndexes))
  (bind _hitresultlist (LocalVariables|GetHitResultList))
  (if (== (Math|Vector|VectorLengthSquared Velocity) 0.0)
    ;[1 1 1] Input velocity is 0, so just short-circut
    (return "0, 0, 0" false (Utilities|Array|MakeArray "") 0 (Utilities|Array|MakeArray 0))
    (else
      (Utilities|FlowControl|Sequence
        (:then_0
          (bind _outvecindirection (CallFunction|GetVecinDirection Velocity DirVec))
          (bind _output_get (LocalVariables|SetVecInDir _outvecindirection))
          (bind (_index0 _index1) (CallFunction|GetBoxDirIndexGivenVector _output_get))
          (LocalVariables|SetRayBoxIndexValues0 _index0)
          (LocalVariables|SetRayBoxIndexValues1 _index1))
        (:then_1
          ;[1 1 1] Get the minimum ray hit distance (i.e. distance to closest hit point) in gravity direction, and check if we will hit.
          (for (_array_element _array_index) (.WasHit (Utilities|Struct|BreakRayBundle (Utilities|Array|Get(acopy) RayCastResults (LocalVariables|GetRayBoxIndexValues0))))
            (if _array_element
              (LocalVariables|SetMinRayHitDistance (Math|Float|Min(Float) (Utilities|Array|Get(acopy) (.RayHitLengths (Utilities|Struct|BreakRayBundle (Utilities|Array|Get(acopy) RayCastResults (LocalVariables|GetRayBoxIndexValues0)))) _array_index) (LocalVariables|GetMinRayHitDistance)))
              (if (<= (Math|Float|Square (Utilities|Array|Get(acopy) (.RayHitLengths (Utilities|Struct|BreakRayBundle (Utilities|Array|Get(acopy) RayCastResults (LocalVariables|GetRayBoxIndexValues0)))) _array_index)) (Math|Vector|VectorLengthSquared (LocalVariables|GetVecInDir)))
                (LocalVariables|SetWasHit true)
                (Utilities|Array|Add (LocalVariables|GetHitResultList) (Utilities|Array|Get(acopy) (.HitResults (Utilities|Struct|BreakRayBundle (Utilities|Array|Get(acopy) RayCastResults (LocalVariables|GetRayBoxIndexValues0)))) _array_index))
                (Utilities|Array|Add (LocalVariables|GetHitResultListRayIndexes) _array_index)
                (LocalVariables|SetHitResultRayBoxIndex (LocalVariables|GetRayBoxIndexValues0))))))
        (:then_2
          (if (LocalVariables|GetWasHit)
            ;[1 1 1] Was hit, so scale the normalized Dir Vec by the hit amount and return that
            (return (* (Math|Vector|Normalize DirVec) (LocalVariables|GetMinRayHitDistance)) true _hitresultlist (LocalVariables|GetHitResultRayBoxIndex) _hitresultlistrayindexes)
            (else
              (return (LocalVariables|GetVecInDir) false _hitresultlist (LocalVariables|GetHitResultRayBoxIndex) _hitresultlistrayindexes))))))))

(fn GetVecinDirection
  (params (InVec :type Vector) (Direction :type Vector))
  (bind _returnvalue (Math|Vector|Normalize Direction))
  (return (* _returnvalue (Math|Vector|DotProduct InVec _returnvalue))))

(fn GetDvDpinDirection
  (params (Direction :type Vector) (InputPin :type Array%20of%20Ray%20Bundle%20Structures) (Velocity :type Vector) (dT :type Float%20%28single-precision%29) (cancelVelocity :type Boolean) (maxVelInDir :type Float%20%28single-precision%29))
  (bind _outvecindirection (CallFunction|GetVecinDirection Velocity Direction))
  (if (> (Math|Vector|VectorLength _outvecindirection) maxVelInDir)
    (LocalVariables|SetvelInDir (* (/ _outvecindirection (Math|Vector|VectorLength _outvecindirection)) maxVelInDir))
    (else
      (LocalVariables|SetvelInDir _outvecindirection)))
  ;[1 1 1] Input says we should just cancel out velocity
  (if cancelVelocity
    (return "0, 0, 0" (* (LocalVariables|GetvelInDir) -1.0) false (Utilities|Array|MakeArray "") 0 (Utilities|Array|MakeArray 0))
    (else
      ;[1 1 1] Handle velocity in gravity direction, and if collision, cancel out velocity in gravity direction.
      (bind _output_get (LocalVariables|SetdP (* (LocalVariables|GetvelInDir) dT)))
      (bind (_ouvelindir _encounteredhit _collisionresultlist _collisionresultrayboxsideindex _collisionresultrayboxsideindexes) (CallFunction|HandleVelocityFunc _output_get Direction InputPin))
      (if _encounteredhit
        (return _ouvelindir (* (LocalVariables|GetvelInDir) -1.5) true _collisionresultlist 0 _collisionresultrayboxsideindexes)
        (else
          (return (LocalVariables|GetdP) "0, 0, 0" false _collisionresultlist _collisionresultrayboxsideindex _collisionresultrayboxsideindexes))))))

(fn GetPerpCounterClockwiseDir
  (params (InVec :type Vector))
  (return (Math|Vector|Normalize (Class|GraviUtilities|GetPerpDirectionCounterClockwise3D InVec))))

(fn HandleTouchInput
  (bind _returnvalue (Transformation|GetActorLocation))
  (bind _draggingtowards (Variables|Default|GetdraggingTowards))
  (bind _gravityvector (Variables|Physics|GetGravityVector))
  (bind _inputstopdelta (Variables|Input|GetInputStopDelta))
  (bind _returnvalue_2 (- _draggingtowards _returnvalue))
  (bind _returnvalue_3 (CallFunction|GetPerpCounterClockwiseDir _gravityvector))
  (bind _returnvalue_4 (Math|Vector|Normalize _returnvalue_3))
  (bind _returnvalue_5 (Math|Vector|DotProduct _returnvalue_4 _returnvalue_2))
  (if (Variables|Default|GetisPlayerDragging)
    ;[1 1 1] This is if the touch event said we should halt, don't try anything then
    (if (Variables|input|GetShouldHaltFromTouchInput)
      (Variables|Input|SetlastDotResult 0.0)
      (return)
      (elif (> _returnvalue_5 _inputstopdelta)
        (Variables|Input|SetRightAmount (Variables|Input|GetMoveSpeed))
        (Variables|input|SetShouldHaltFromTouchInput false)
        (elif (< _returnvalue_5 (* _inputstopdelta -1.0))
          (Variables|Input|SetRightAmount (* (Variables|Input|GetMoveSpeed) -1.0))
          (Variables|input|SetShouldHaltFromTouchInput false)
          (else
            (Variables|input|SetShouldHaltFromTouchInput true)))))
    (else
      (Variables|input|SetShouldHaltFromTouchInput true)))
  (if (< (* (Variables|Input|GetlastDotResult) _returnvalue_5) 0.0)
    (Variables|input|SetShouldHaltFromTouchInput true))
  (Variables|Input|SetlastDotResult _returnvalue_5))

(fn GetRayBoxCorners
  (params (RayBox :type Scene%20Component%20Object%20Reference))
  (bind (_origin _boxextent) (Collision|GetComponentBounds RayBox))
  (bind (_origin_2 _boxextent_2) (Collision|GetComponentBounds RayBox))
  (bind (_origin_3 _boxextent_3) (Collision|GetComponentBounds RayBox))
  (bind (_origin_4 _boxextent_4) (Collision|GetComponentBounds RayBox))
  (bind (_x _y _z) (Math|Vector|BreakVector _boxextent_4))
  (bind (_x_2 _y_2 _z_2) (Math|Vector|BreakVector _boxextent_2))
  (return (Utilities|Array|MakeArray (- _origin _boxextent) (+ _origin_2 (Math|Vector|MakeVector _x_2 0.0 (* _z_2 -1.0))) (+ _origin_3 _boxextent_3) (+ _origin_4 (Math|Vector|MakeVector (* _x -1.0) 0.0 _z)))))

(fn HandleHitwithSpecialObjects
  (params (Hit :type Hit%20Result%20Structure%20%28by%20ref%29))
  (bind (_bblockinghit _binitialoverlap _time _location _impactpoint _normal _impactnormal _physmat _hitactor) (Collision|BreakHitResult Hit))
  (bind _returnvalue (Actor|GetComponentbyClass _hitactor "/Script/Paper2D.PaperTileMapComponent"))
  ;[1 1 1] Get the colliding tile
  (if (Utilities|ClassIsChildOf (Utilities|GetClass _hitactor) "/Script/Paper2D.PaperTileMapActor")
    (bind (_outtilex _outtiley) (Class|AdvancedTileMapComponent|GetTileCoordinatesfromLocalSpacePosition _returnvalue (Math|Transform|InverseTransformLocation (Transformation|GetActorTransform _hitactor) (+ _impactpoint (* _normal -1.0)))))
    (CallFunction|TileCollisionEvent (Class|PaperTileMapComponent|GetTile _returnvalue _outtilex _outtiley) _returnvalue)
    (Development|PrintString (Utilities|String|ToString(Integer) _outtilex) true true "(R=0.000000,G=1.000000,B=0.114498,A=1.000000)")
    (Development|PrintString (Utilities|String|ToString(Integer) _outtiley) true true "(R=0.131993,G=1.000000,B=0.000000,A=1.000000)")
    (else
      ;[1 1 1] Handle hitting the game levelgoal, call PlayerLevelGoal event
      (if (Utilities|ClassIsChildOf (Utilities|GetClass _hitactor) "/Game/Blueprints/LevelObjects/LevelGoal.LevelGoal_C")
        (bind _aslevel_goal (Utilities|Casting|CastToLevelGoal _hitactor))
        (CallFunction|PlayerLevelGoal _aslevel_goal)))))