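; Player controller for a gravity puzzle game that turns touch input into level rotation or player dragging.
; Dragging on the LevelControl rotates the level camera by the signed angle around the tilemap's screen center, with the background copying the camera's rotation, while physics is paused.
; On release it snaps to quarter turns, broadcasts the new gravity direction and resumes physics.
; Touches on GraviPlayer are forwarded to its touch handlers.
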(event EventBeginPlay
  (Variables|/Script/Engine.PlayerController|SetbEnableClickEvents (Game|GetPlayerController 0) true)
  (Variables|Default|SetbEnableMouseOverEvents true)
  (bind _outactors (Actor|GetAllActorsOfClass "/Game/Blueprints/Cameras/MyCamera.MyCamera_C"))
  (Game|Player|SetViewTargetwithBlend (Game|GetPlayerController 0) (Utilities|Array|Get(acopy) _outactors) 0.0 "VTBlend_Linear" 0.0 false)
  ;[1 1 1] Set GraviPlayer variable
  (bind _asgravi_player (Utilities|Casting|CastToGraviPlayer (Game|GetPlayerCharacter 0)))
  (Variables|Default|SetGraviPlayer _asgravi_player)
  ;[1 1 1] Set the level info from the game mode
  (bind _asmy_game_mode (Utilities|Casting|CastToMyGameMode (Game|GetGameMode))
    (:then
      (Variables|Default|SetGameMode _asmy_game_mode)
      ;[1 1 1] Level background
      (bind _outactors_2 (Actor|GetAllActorsOfClass "/Game/Blueprints/LevelObjects/Backgrounds/DefaultLevelBackground.DefaultLevelBackground_C"))
      ;;[1 1 1] If we have this background.  If not, this will be set up on demand later in the event graph
      (if (> (Utilities|Array|Length _outactors_2) 0)
        (bind _asdefault_level_background (Utilities|Casting|CastToDefaultLevelBackground (Utilities|Array|Get(acopy) _outactors_2))
          (:then
            (Variables|Default|SetLevelBackgroundRef _asdefault_level_background))
          (:CastFailed
            (Development|PrintString "NO LEVEL BACKGROUND ACTOR!")))))
    (:CastFailed
      (Development|PrintString "FAILED TO GET MY GAME MODE!!"))))

(event EventTick
  (params (DeltaSeconds :type Float%20%28single-precision%29)))

(event Input|TouchEvents|InputTouch
  (params (Location :type Vector) (FingerIndex :type ETouchIndex%20Enum))
  (bind _returnvalue (Game|GetPlayerController 0))
  (bind _returnvalue_2 (Game|GetPlayerController 0))
  (bind (_x _y) (Math|Vector|BreakVector Location))
  (bind _gamemode (Variables|Default|GetGameMode))
  (bind _gamemode_2 (Variables|Default|GetGameMode))
  (bind _graviplayer (Variables|Default|GetGraviPlayer))
  (bind _gamemode_3 (Variables|Default|GetGameMode))
  (bind _hitresult (Class|PlayerController|GetHitResultUnderFingerbyChannel _returnvalue "Touch1" "TraceTypeQuery1" true))
  (bind _returnvalue_3 (Math|Vector2D|MakeVector2D _x _y))
  (bind _levelinfo (Variables|/Game/Blueprints/Utilities/MyGameMode.MyGameMode_C|GetLevelInfo _gamemode))
  (bind _isplayerdragging (Variables|/Game/Blueprints/Player/GraviPlayer.GraviPlayer_C|GetisPlayerDragging _graviplayer))
  (bind _levelinfo_2 (Variables|/Game/Blueprints/Utilities/MyGameMode.MyGameMode_C|GetLevelInfo _gamemode_2))
  (bind _levelinfo_3 (Variables|/Game/Blueprints/Utilities/MyGameMode.MyGameMode_C|GetLevelInfo _gamemode_3))
  (bind _hitactor (Collision|BreakHitResult _hitresult))
  (bind _levelcamera (Variables|/Game/Blueprints/Utilities/LevelInfo.LevelInfo_C|GetLevelCamera _levelinfo))
  (bind _tilemapref (Variables|/Game/Blueprints/Utilities/LevelInfo.LevelInfo_C|GetTileMapRef _levelinfo_2))
  (bind _levelcamera_2 (Variables|/Game/Blueprints/Utilities/LevelInfo.LevelInfo_C|GetLevelCamera _levelinfo_3))
  (bind _rendercomponent (Variables|/Script/Paper2D.PaperTileMapActor|GetRenderComponent _tilemapref))
  (bind _origin (Collision|GetComponentBounds _rendercomponent))
  (bind _screenposition (Class|GameplayStatics|ProjectWorldtoScreen _returnvalue_2 _origin false))
  (bind _returnvalue_4 (- _returnvalue_3 _screenposition))
  (bind _returnvalue_5 (Math|Vector2D|Normalize2D _returnvalue_4))
  (bind (_x_2 _y_2) (Math|Vector2D|BreakVector2D _returnvalue_5))
  (:Pressed
    (Utilities|Casting|CastToLevelControl _hitactor
      (:then
        (Variables|RotationControls|SetTileMapIsDragging true)
        (Variables|RotationControls|SetrcStartTouchPos _returnvalue_3)
        (Default|CallPausePhysicsDispatcher true))
      (:CastFailed
        ;[1 1 1] Handle player touch events
        (bind _asgravi_player (Utilities|Casting|CastToGraviPlayer _hitactor))
        (Default|GraviTouchPressed _asgravi_player))))
  (:Released
    (if _isplayerdragging
      (Default|GraviTouchReleased _asgravi_player)
      (elif (Variables|RotationControls|GetTileMapIsDragging)
        (Variables|RotationControls|SetTileMapIsDragging false)
        ;[1 1 1] Quantize the angle to one of -180, -90, 0, 90, 180
        (bind _output_get (Variables|RotationControls|SetrcOffsetRotation (Math|Conversions|ToFloat(Integer) (Math|Integer|Clamp(Integer) (- (* (Class|KismetSystemLibrary|MakeLiteralInteger (Math|Float|Truncate (/ (+ (Variables|RotationControls|GetrcLastRotation) 225.0) 9e+01))) 90) 180) -180 180))))
        (Transformation|SetActorRotation _levelcamera_2 (Math|Rotator|MakeRotator 0.0 _output_get 0.0))
        (CallFunction|SetBackgroundRotation _levelcamera_2)
        (Utilities|FlowControl|Sequence
          (:then_0
            (if (== _output_get 0.0)
              (Default|CallChangeGravityDirectionDispatcher "(X=0.000000,Y=-1.000000)")
              (elif (== _output_get 9e+01)
                (Default|CallChangeGravityDirectionDispatcher "(X=1.000000,Y=0.000000)")
                (elif (or (== _output_get 1.8e+02) (== _output_get -1.8e+02))
                  (Default|CallChangeGravityDirectionDispatcher "(X=0.000000,Y=1.000000)")
                  (elif (== _output_get -9e+01)
                    (Default|CallChangeGravityDirectionDispatcher "(X=-1.000000,Y=0.000000)")
                    (else
                      (Development|PrintString "UNKNOWN GRAVITY ROTATION!" true true "(R=1.000000,G=0.029236,B=0.088960,A=1.000000)")))))))
          (:then_1
            (Default|CallPausePhysicsDispatcher false))))))
  (:Moved
    (if _isplayerdragging
      (Default|GraviTouchMoved _asgravi_player Location)
      (elif (Variables|RotationControls|GetTileMapIsDragging)
        ;[1 1 1] rotate the camera
        (Transformation|SetActorRotation _levelcamera (Math|Rotator|MakeRotator 0.0 (CallFunction|ConvertAngle (+ (* (Class|KismetMathLibrary|DegAtan2 (- (* _x_2 (.Y (Math|Vector2D|BreakVector2D (Math|Vector2D|Normalize2D (- (Variables|RotationControls|GetrcStartTouchPos) _screenposition))))) (* _y_2 (.X (Math|Vector2D|BreakVector2D (Math|Vector2D|Normalize2D (- (Variables|RotationControls|GetrcStartTouchPos) _screenposition)))))) (Math|Vector2D|DotProduct(2D) _returnvalue_5 (Math|Vector2D|Normalize2D (- (Variables|RotationControls|GetrcStartTouchPos) _screenposition)))) -1.0) (Variables|RotationControls|GetrcOffsetRotation))) 0.0))
        (Variables|RotationControls|SetrcLastRotation (CallFunction|ConvertAngle (+ (* (Class|KismetMathLibrary|DegAtan2 (- (* _x_2 (.Y (Math|Vector2D|BreakVector2D (Math|Vector2D|Normalize2D (- (Variables|RotationControls|GetrcStartTouchPos) _screenposition))))) (* _y_2 (.X (Math|Vector2D|BreakVector2D (Math|Vector2D|Normalize2D (- (Variables|RotationControls|GetrcStartTouchPos) _screenposition)))))) (Math|Vector2D|DotProduct(2D) _returnvalue_5 (Math|Vector2D|Normalize2D (- (Variables|RotationControls|GetrcStartTouchPos) _screenposition)))) -1.0) (Variables|RotationControls|GetrcOffsetRotation))))
        (CallFunction|SetBackgroundRotation _levelcamera)))))

(fn ConstructionScript)

(fn ConvertAngle
  (params (angle :type Float%20%28single-precision%29))
  (if (> angle 1.8e+02)
    (return (- angle 3.6e+02))
    (elif (< angle -1.8e+02)
      (return (+ angle 3.6e+02))
      (else
        (return angle)))))

(fn SetBackgroundRotation
  (params (CameraActorRef :type Actor%20Object%20Reference))
  ;[1 1 1] Rotate background in opposite direction
  (Utilities|IsValid (Variables|Default|GetLevelBackgroundRef)
    (:Is%20Valid
      _)
    (:Is%20Not%20Valid
      (bind _outactors (Actor|GetAllActorsOfClass "/Game/Blueprints/LevelObjects/Backgrounds/DefaultLevelBackground.DefaultLevelBackground_C"))
      (Variables|Default|SetLevelBackgroundRef (Utilities|Array|Get(acopy) _outactors))))
  (Transformation|SetActorRotation (Variables|Default|GetLevelBackgroundRef) (Transformation|GetActorRotation CameraActorRef)))