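; A 2D level block whose PhysicalRayboxBP is constrained to a rail between two endpoints defined relative to the root.
; The construction script creates collision-free Paper2D sprites for both endpoints and the rail.
; The rail sprite is centred and Z-scaled to the endpoint distance, with a dynamic material "Vscale" set to the same ratio.
; BeginPlay derives the constraint vector, center and half-length, and Tick pins the sprites at cached world positions.
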(event EventBeginPlay
  (bind _physicalrayboxbp (Variables|Default|GetPhysicalRayboxBP))
  (|CallParentFunction)
  (bind (_endpoint1worldloc _endpoint2worldloc) (CallFunction|SetEndpointSpriteLocations))
  (Utilities|FlowControl|Sequence
    (:then_0
      (Variables|/Game/Blueprints/Components/PhysicalRayboxBP.PhysicalRayboxBP_C|SetConstrainToVector _physicalrayboxbp (- _endpoint2worldloc _endpoint1worldloc))
      (Variables|/Game/Blueprints/Components/PhysicalRayboxBP.PhysicalRayboxBP_C|SetConstrainToVectorCenter _physicalrayboxbp (+ (* (- _endpoint1worldloc _endpoint2worldloc) 0.5) _endpoint2worldloc))
      (Variables|/Game/Blueprints/Components/PhysicalRayboxBP.PhysicalRayboxBP_C|SetConstrainToVectorLength _physicalrayboxbp (Math|Vector2D|Vector2DLength (* (- _endpoint1worldloc _endpoint2worldloc) 0.5))))
    (:then_1
      (Variables|RailProperties|SetinternalRailEndpoint1 (Class|GraviUtilities|Get3DVector _endpoint1worldloc 0.0))
      (Variables|RailProperties|SetinternalRailEndpoint2 (Class|GraviUtilities|Get3DVector _endpoint2worldloc 0.0)))))

(event Collision|EventActorBeginOverlap
  (params (OtherActor :type Actor%20Object%20Reference)))

(event EventTick
  (params (DeltaSeconds :type Float%20%28single-precision%29))
  (|CallParentFunction DeltaSeconds)
  (Transformation|SetWorldLocation (Variables|RailProperties|GetrailEnpoint1SpriteSceneComponentRef) (Variables|RailProperties|GetinternalRailEndpoint1) false false)
  (Transformation|SetWorldLocation (Variables|RailProperties|GetrailEnpoint2SpriteSceneComponentRef_0) (Variables|RailProperties|GetinternalRailEndpoint2) false false)
  (Transformation|SetWorldLocation (Variables|RailProperties|GetrailSpriteComponent) (Variables|RailProperties|GetinternalRailPosition) false false))

(fn ConstructionScript
  (|CallParentFunction)
  (bind _returnvalue (AddComponent|AddPaperSpriteComponent false))
  (Collision|SetCollisionEnabled _returnvalue "NoCollision")
  (Rendering|Components|Sprite|SetSprite _returnvalue (Variables|RailProperties|GetRailEndpointSprite))
  (Variables|RailProperties|SetrailEnpoint1SpriteSceneComponentRef _returnvalue)
  (bind _returnvalue_2 (AddComponent|AddPaperSpriteComponent false))
  (Collision|SetCollisionEnabled _returnvalue_2 "NoCollision")
  (Rendering|Components|Sprite|SetSprite _returnvalue_2 (Variables|RailProperties|GetRailEndpointSprite))
  (Variables|RailProperties|SetrailEnpoint2SpriteSceneComponentRef_0 _returnvalue_2)
  (bind _returnvalue_3 (AddComponent|AddPaperSpriteComponent false))
  (Collision|SetCollisionEnabled _returnvalue_3 "NoCollision")
  (Rendering|Components|Sprite|SetSprite _returnvalue_3 (Variables|RailProperties|GetRailSprite))
  (Variables|RailProperties|SetrailSpriteComponent _returnvalue_3)
  (Transformation|SetAbsolute (Variables|RailProperties|GetrailEnpoint1SpriteSceneComponentRef) false false true)
  (Transformation|SetAbsolute (Variables|RailProperties|GetrailEnpoint2SpriteSceneComponentRef_0) false false true)
  (Transformation|SetAbsolute (Variables|RailProperties|GetrailSpriteComponent) false false true)
  (Variables|RailProperties|SetinternalRailOriginalBoxExtents (.BoxExtent (Collision|GetComponentBounds (Variables|RailProperties|GetrailSpriteComponent))))
  (CallFunction|SetEndpointSpriteLocations))

(fn SetEndpointSpriteLocations
  (bind _output_get (Variables|RailProperties|SetinternalRailEndpoint1 (Class|GraviUtilities|Get3DVector (Class|GraviUtilities|Get2DVector (Math|Transform|TransformLocation (Transformation|GetWorldTransform (Variables|Default|GetDefaultSceneRoot)) (Variables|RailProperties|GetRailEndpoint1))) -1.0)))
  (Transformation|SetWorldLocation (Variables|RailProperties|GetrailEnpoint1SpriteSceneComponentRef) _output_get false false)
  (bind _output_get_2 (Variables|RailProperties|SetinternalRailEndpoint2 (Class|GraviUtilities|Get3DVector (Class|GraviUtilities|Get2DVector (Math|Transform|TransformLocation (Transformation|GetWorldTransform (Variables|Default|GetDefaultSceneRoot)) (Variables|RailProperties|GetRailEndpoint2))) -1.0)))
  (Transformation|SetWorldLocation (Variables|RailProperties|GetrailEnpoint2SpriteSceneComponentRef_0) _output_get_2 false false)
  (CallFunction|SetRailSpriteParameters (Class|GraviUtilities|Get2DVector _output_get) (Class|GraviUtilities|Get2DVector _output_get_2))
  (return (Class|GraviUtilities|Get2DVector _output_get) (Class|GraviUtilities|Get2DVector _output_get_2)))

(fn SetRailSpriteParameters
  (params (endpoint1 :type Vector%202D%20Structure) (endpoint2 :type Vector%202D%20Structure))
  (bind _returnvalue (- endpoint1 endpoint2))
  (bind _railspritecomponent (Variables|RailProperties|GetrailSpriteComponent))
  (bind _internalrailoriginalboxextents (Variables|RailProperties|GetinternalRailOriginalBoxExtents))
  (bind _returnvalue_2 (Math|Vector2D|Vector2DLength _returnvalue))
  (bind _z (Math|Vector|BreakVector _internalrailoriginalboxextents))
  (bind _returnvalue_3 (Transformation|GetWorldScale _railspritecomponent))
  (bind _returnvalue_4 (* _returnvalue 0.5))
  (bind (_x _y) (Math|Vector|BreakVector _returnvalue_3))
  (bind _returnvalue_5 (* _z 2.0))
  (bind _returnvalue_6 (+ _returnvalue_4 endpoint2))
  (bind _returnvalue_7 (/ _returnvalue_2 _returnvalue_5))
  (bind _returnvalue_8 (Class|GraviUtilities|Get3DVector _returnvalue_6 0.0))
  (bind _returnvalue_9 (Rendering|Material|CreateDynamicMaterialInstance _railspritecomponent 0 (Rendering|Material|GetMaterial _railspritecomponent 0) :!class /Script/Engine.PrimitiveComponent))
  (Rendering|Material|SetMaterial _railspritecomponent 0 _returnvalue_9)
  (Rendering|Material|SetScalarParameterValue _returnvalue_9 "Vscale" _returnvalue_7 :!class /Script/Engine.MaterialInstanceDynamic)
  (Transformation|SetWorldScale3D _railspritecomponent (Math|Vector|MakeVector _x _y _returnvalue_7))
  (Transformation|SetWorldLocation _railspritecomponent _returnvalue_8 false false)
  (Variables|RailProperties|SetinternalRailPosition _returnvalue_8))