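; Block is a sprite-based level object that moves under gravity with minimal bounce through a custom raybox physics component.
; Each Tick configures PhysicalRayboxBP with the box collision and runs it.
; Its physics update dispatcher returns a position delta, applied as an unswept actor offset converted to 3D with zero Y.
; The construction script creates a dynamic border material and feeds it the sprite's world X and Z scale as U and V scale.
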(event Custom|PhysicsUpdate
  (params (newVelocity :type Vector%202D%20Structure) (deltaPosition :type Vector%202D%20Structure))
  (Transformation|AddActorWorldOffset (Class|GraviUtilities|Get3DVector deltaPosition 0.0)))

(event EventBeginPlay
  (EventDispatchers|BindEventtoPhysicsUpdateDispatcher (Variables|Default|GetPhysicalRayboxBP) (delegate Custom|PhysicsUpdate)))

(event Collision|EventActorBeginOverlap
  (params (OtherActor :type Actor%20Object%20Reference)))

(event EventTick
  (params (DeltaSeconds :type Float%20%28single-precision%29))
  (bind _physicalrayboxbp (Variables|Default|GetPhysicalRayboxBP))
  (Variables|/Game/Blueprints/Components/PhysicalRayboxBP.PhysicalRayboxBP_C|SetRayBoxGeo _physicalrayboxbp (Variables|Default|GetBoxCollision))
  (Variables|/Game/Blueprints/Components/PhysicalRayboxBP.PhysicalRayboxBP_C|SetConstrainToGravity _physicalrayboxbp true)
  (Variables|/Game/Blueprints/Components/PhysicalRayboxBP.PhysicalRayboxBP_C|SetBounciness _physicalrayboxbp 0.01)
  (Default|DoTick _physicalrayboxbp DeltaSeconds))

(fn ConstructionScript
  (CallFunction|SetupBlockMaterialParams))

(fn SetupBlockMaterialParams
  (bind _blocksprite (Variables|Default|GetBlockSprite))
  (bind _blocksprite_2 (Variables|Default|GetBlockSprite))
  (bind _returnvalue (Transformation|GetWorldScale _blocksprite))
  (bind (_x _y _z) (Math|Vector|BreakVector _returnvalue))
  (bind _returnvalue_2 (Rendering|Material|CreateDynamicMaterialInstance _blocksprite_2 0 "/Game/Materials/BorderMaterialInstance.BorderMaterialInstance" :!class /Script/Engine.PrimitiveComponent))
  (Rendering|Material|SetMaterial _blocksprite_2 0 _returnvalue_2)
  (Rendering|Material|SetScalarParameterValue _returnvalue_2 "Vscale" _z :!class /Script/Engine.MaterialInstanceDynamic)
  (Rendering|Material|SetScalarParameterValue _returnvalue_2 "Uscale" _x :!class /Script/Engine.MaterialInstanceDynamic))