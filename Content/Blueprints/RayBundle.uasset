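; RayBundle casts evenly spaced line traces from the four sides of a box in the X-Z plane.
; BeginPlay fills BoxWorldCorners with zero vectors, which CastRays reads as consecutive pairs to form each side.
; Rays follow each side's perpendicular from an offset start, using the Visibility channel with debug drawing.
; CastRays returns per-side hit results, hit flags and offset-corrected hit lengths.
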(event EventBeginPlay
  ;[1 1 1] Sets up the ray bundle with default values
  (CallFunction|SetupRayBundle))

(event EventTick
  (params (DeltaSeconds :type Float%20%28single-precision%29)))

(fn SetupRayBundle
  ;[1 1 1] Creates four corners in the array, clearing any previous values
  (Utilities|Array|Clear (Variables|Default|GetBoxWorldCorners))
  (for _index (range 0 4)
    (Utilities|Array|Add (Variables|Default|GetBoxWorldCorners) (Math|Vector|MakeVector 0.0 0.0 0.0))))

(fn CastRays
  (bind _returnrays (LocalVariables|GetReturnRays))
  (bind _returnrays_2 (LocalVariables|GetReturnRays))
  (bind _raystartoffset (Variables|Default|GetRayStartOffset))
  (bind (_hitresults _washit _rayhitlengths) (Utilities|Struct|BreakRayBundleResults _returnrays_2))
  (bind (_hitresults_2 _washit_2) (Utilities|Struct|BreakRayBundleResults _returnrays))
  (bind _returnvalue (* _raystartoffset -1.0))
  (Utilities|Array|Clear (LocalVariables|GetReturnRaysArray))
  ;[1 1 1] For each of the sides of the box
  (for _index (range 0 3)
    (Utilities|FlowControl|Sequence
      (:then_0
        ;[1 1 1] Make sure array is 2 large
        (Utilities|Array|Resize (LocalVariables|GetCurrentSideBounds) 2)
        ;[1 1 1] Set the local CurrentRayStarts[0] and [1] to be the current ray starts.
        (Utilities|FlowControl|Sequence
          (:then_0
            (Utilities|Array|SetArrayElem (LocalVariables|GetCurrentSideBounds) 0 (Utilities|Array|Get(acopy) (Variables|Default|GetBoxWorldCorners) _index)))
          (:then_1
            (Utilities|Array|SetArrayElem (LocalVariables|GetCurrentSideBounds) 1 (Utilities|Array|Get(acopy) (Variables|Default|GetBoxWorldCorners) (Math|Integer|%(Integer) (+ _index 1) 4))))))
      (:then_1
        ;[1 1 1] Create CurrentRayStartsDiff vector from CurrentRayStarts[0] to CurrentRayStarts[1].  Also Creates the normal (rays' direction)
        (bind _output_get (LocalVariables|SetCurrentRayStartsDiff (- (Utilities|Array|Get(acopy) (LocalVariables|GetCurrentSideBounds) 1) (Utilities|Array|Get(acopy) (LocalVariables|GetCurrentSideBounds)))))
        (bind _normvector (Utility|Get2DVectorNormal _output_get))
        (LocalVariables|SetCurrentRayStartsNorm _normvector))
      (:then_2
        ;[1 1 1] Fill local variable ReturnArrays with hit results
        ;;[1 1 1] Clear any previous results of ReturnRays
        (Utilities|Array|Clear _hitresults_2)
        (Utilities|Array|Clear _washit_2)
        ;;[1 1 1] Loop through each ray on this side
        (for _index_2 (range 0 (- (Variables|Default|GetNumRaysPerSide) 1))
          (Rendering|Debug|DrawDebugCircle (+ (+ (Utilities|Array|Get(acopy) (LocalVariables|GetCurrentSideBounds)) (* (LocalVariables|GetCurrentRayStartsDiff) (/ (Math|Conversions|ToFloat(Integer) _index_2) (Math|Conversions|ToFloat(Integer) (- (Variables|Default|GetNumRaysPerSide) 1))))) (* (LocalVariables|GetCurrentRayStartsNorm) (Variables|Default|GetRayStartOffset))) 1e+01 12 "(R=0.000000,G=0.086107,B=1.000000,A=1.000000)" 0.0 1.0 "0.000000,1.000000,1.000000" "1.000000,0.000000,1.000000")
          (bind (_outhit _returnvalue_2) (Collision|LineTraceByChannel (+ (+ (Utilities|Array|Get(acopy) (LocalVariables|GetCurrentSideBounds)) (* (LocalVariables|GetCurrentRayStartsDiff) (/ (Math|Conversions|ToFloat(Integer) _index_2) (Math|Conversions|ToFloat(Integer) (- (Variables|Default|GetNumRaysPerSide) 1))))) (* (LocalVariables|GetCurrentRayStartsNorm) (Variables|Default|GetRayStartOffset))) (+ (+ (Utilities|Array|Get(acopy) (LocalVariables|GetCurrentSideBounds)) (* (LocalVariables|GetCurrentRayStartsDiff) (/ (Math|Conversions|ToFloat(Integer) _index_2) (Math|Conversions|ToFloat(Integer) (- (Variables|Default|GetNumRaysPerSide) 1))))) (* (LocalVariables|GetCurrentRayStartsNorm) (Variables|Default|GetRayLengths))) "TraceTypeQuery1" false 0 "ForOneFrame"))
          (Utilities|Array|Add _hitresults _outhit)
          ;;[1 1 1] Subtract the offset value
          (Utilities|Array|Add _washit _returnvalue_2)
          (if _returnvalue_2
            (Utilities|Array|Add _rayhitlengths (- (* (.Time (Collision|BreakHitResult _outhit)) (+ (Variables|Default|GetRayLengths) _returnvalue)) _returnvalue))
            (else
              (Utilities|Array|Add _rayhitlengths (Math|Float|MakeLiteralFloat 0.0))))))
      (:then_3
        ;[1 1 1] Add to the ReturnRaysArray
        (Utilities|Array|Add (LocalVariables|GetReturnRaysArray) (LocalVariables|GetReturnRays)))))
  ;[1 1 1] Return results
  (return (LocalVariables|GetReturnRaysArray)))

(fn Get2DVectorNormal
  (params (inVector :type Vector))
  (bind (_x _y _z) (Math|Vector|BreakVector inVector))
  (return (Math|Vector|Normalize (Math|Vector|MakeVector _z 0.0 (* _x -1.0)))))