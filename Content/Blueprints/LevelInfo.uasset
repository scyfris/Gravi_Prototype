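; LevelInfo is a level manager actor that rotates the view and player gravity in a game with a rotatable level.
; Its construction script caches the first MyCamera and Player actors and registers itself on the player.
; DoRotateLevel calls RotateLevel, which steps the angle by 90 degrees and applies it as camera pitch.
; Only down-right rotation turns the player's GravityVector in the XZ plane; down-left resets non-positive angles to zero.
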(event Custom|DoRotateLevel
  (params (RotateEnum :type LevelRotationEnum%20Enum))
  (CallFunction|RotateLevel RotateEnum))

(event EventBeginPlay)

(event Collision|EventActorBeginOverlap
  (params (OtherActor :type Actor%20Object%20Reference)))

(event EventTick
  (params (DeltaSeconds :type Float%20%28single-precision%29)))

(fn ConstructionScript
  (Utilities|FlowControl|Sequence
    (:then_0
      ;[1 1 1] Sets the current camera to the level's camera
      (bind _outactors (Actor|GetAllActorsOfClass "/Game/Blueprints/MyCamera.MyCamera_C"))
      (Variables|GlobalActorRefs|SetLevelCamera (Utilities|Array|Get(acopy) _outactors)))
    (:then_1
      ;[1 1 1] Set up the player references
      (bind _outactors_2 (Actor|GetAllActorsOfClass "/Game/Blueprints/Player.Player_C"))
      (bind _asplayer (Utilities|Casting|CastToPlayer (Utilities|Array|Get(acopy) _outactors_2))
        (:then
          (Variables|/Game/Blueprints/Player.Player_C|SetLevelInfoRef _asplayer self)
          (Variables|GlobalActorRefs|SetPlayerRef _asplayer))
        (:CastFailed
          (Class|VisualLoggerKismetLibrary|LogText "Can't get player!!!" "Blueprint Log"))))))

(fn RotateLevel
  (params (RotationDir :type LevelRotationEnum%20Enum))
  (bind _playerref (Variables|GlobalActorRefs|GetPlayerRef))
  (Utilities|FlowControl|Sequence
    (:then_0
      ;[1 1 1] SetCurrentRotation based on rotation input enum
      (switch Utilities|FlowControl|Switch|SwitchonLevelRotationEnum RotationDir
        (:NewEnumerator0
          (bind _output_get (Variables|RotationInfo|SetCurrentRotation (+ (Variables|RotationInfo|GetCurrentRotation) 90)))
          (if (>= _output_get 360)
            (Variables|RotationInfo|SetCurrentRotation 0)))
        (:NewEnumerator1
          (bind _output_get_2 (Variables|RotationInfo|SetCurrentRotation (+ (Variables|RotationInfo|GetCurrentRotation) -90)))
          (if (<= _output_get_2 0)
            (Variables|RotationInfo|SetCurrentRotation 0)))))
    (:then_1
      ;[1 1 1] rotate the camera
      (Transformation|SetActorRotation (Variables|GlobalActorRefs|GetLevelCamera) (Math|Rotator|MakeRotator 0.0 (Math|Conversions|ToFloat(Integer) (Variables|RotationInfo|GetCurrentRotation)) 0.0)))
    (:then_2
      (switch Utilities|FlowControl|Switch|SwitchonLevelRotationEnum RotationDir
        (:NewEnumerator0
          (Variables|/Game/Blueprints/Player.Player_C|SetGravityVector _playerref (Math|Vector|MakeVector (* (.Z (Math|Vector|BreakVector (Variables|/Game/Blueprints/Player.Player_C|GetGravityVector _playerref))) -1.0) 0.0 (.X (Math|Vector|BreakVector (Variables|/Game/Blueprints/Player.Player_C|GetGravityVector _playerref))))))))))