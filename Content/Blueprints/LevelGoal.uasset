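; LevelGoal is an actor for a level goal, shown as a gem sprite with a GoalSystem particle effect.
; On BeginPlay a hover timeline starts, adding its position value to the sprite's local offset each update.
; The same update sets the particles' initial velocity to a random X and the negated timeline Z, opposing the hover motion.
; Clicking the gem only prints a debug string, and no goal-reached logic is implemented.
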(event OnClicked(gems_db16_Sprite_4)
  (params (TouchedComponent :type Primitive%20Component%20Object%20Reference) (ButtonPressed :type Key%20Structure :default "AnyKey"))
  (Development|PrintString "Hello"))

(event EventBeginPlay
  (bind _positionanimation (Timeline|HoverTimeline PlayFromStart)
    (:Update
      (Transformation|AddLocalOffset (Variables|Default|Getgems_db16_Sprite_4) _positionanimation false false)
      (Effects|Components|ParticleSystem|SetVectorParameter (Variables|Default|GetGoalSystem) "initialVelocity" (Math|Vector|MakeVector (Math|Random|RandomFloat) 0.0 (* (.Z (Math|Vector|BreakVector _positionanimation)) -1.0))))))

(event Collision|EventActorBeginOverlap
  (params (OtherActor :type Actor%20Object%20Reference)))

(event EventTick
  (params (DeltaSeconds :type Float%20%28single-precision%29)))

(fn ConstructionScript)