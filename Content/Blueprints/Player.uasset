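; Player Blueprint for movement in the X-Z plane with hand-rolled gravity and collision, plus an input that asks the level info object to rotate the level.
; Each tick it casts a ray bundle from the RayBox corners and feeds the hits to UpdatePhysics.
; Velocity splits along gravity and its perpendicular; hits clamp displacement and cancel that component before an unswept actor offset.
; A second Move handler uses AddMovementInput behind an unfinished ledge trace starting at world origin.
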(event EventBeginPlay
  ;[1 1 1] Events
)

(event Collision|EventActorBeginOverlap
  (params (OtherActor :type Actor%20Object%20Reference))
  ;[1 1 1] Events
)

(event EventTick
  (params (DeltaSeconds :type Float%20%28single-precision%29))
  (bind _raybox (Variables|Default|GetRayBox))
  (bind _raybox_2 (Variables|Default|GetRayBox))
  (bind _raybox_3 (Variables|Default|GetRayBox))
  (bind _raybox_4 (Variables|Default|GetRayBox))
  (bind (_origin _boxextent) (Collision|GetComponentBounds _raybox))
  (bind (_origin_2 _boxextent_2) (Collision|GetComponentBounds _raybox_2))
  (bind (_origin_3 _boxextent_3) (Collision|GetComponentBounds _raybox_3))
  (bind (_origin_4 _boxextent_4) (Collision|GetComponentBounds _raybox_4))
  (bind (_x _y _z) (Math|Vector|BreakVector _boxextent))
  (bind (_x_2 _y_2 _z_2) (Math|Vector|BreakVector _boxextent_4))
  ;[1 1 1] Events
  (Utilities|FlowControl|Sequence
    (:then_0
      ;[1 1 1] Cast the rays!
      (Variables|/Game/Blueprints/RayBundle.RayBundle_C|SetBoxWorldCorners (Variables|Default|GetRayBundle) (Utilities|Array|MakeArray (- _origin_3 _boxextent_3) (+ _origin_4 (Math|Vector|MakeVector _x_2 0.0 (* _z_2 -1.0))) (+ _origin_2 _boxextent_2) (+ _origin (Math|Vector|MakeVector (* _x -1.0) 0.0 _z))))
      ;[1 1 1] Raybundle setup
      ;;[1 1 1] Set the initial ray lengths.
      (Variables|/Game/Blueprints/RayBundle.RayBundle_C|SetRayLengths (Variables|Default|GetRayBundle) (Variables|RayBoxInfo|GetRayBoxRayLength))
      ;;[1 1 1] Set the ray offsets
      (Variables|/Game/Blueprints/RayBundle.RayBundle_C|SetRayStartOffset (Variables|Default|GetRayBundle) (Variables|RayBoxInfo|GetRayBoxOffsets))
      ;;[1 1 1] Set the number of rays per side
      (Variables|/Game/Blueprints/RayBundle.RayBundle_C|SetNumRaysPerSide (Variables|Default|GetRayBundle) (Variables|RayBoxInfo|GetRayBoxNumPerSide))
      (bind _returnbundles (Default|CastRays (Variables|Default|GetRayBundle)))
      (CallFunction|UpdatePhysics DeltaSeconds _returnbundles))))

(event Input|ActionEvents|InputActionRotateRightDown
  (params (Key :type Key%20Structure :default "AnyKey"))
  (:Pressed
    (Default|RotateLevel (Variables|ExternalRefs|GetLevelInfoRef) "NewEnumerator0")))

(event Input|AxisEvents|InputAxisMove
  (params (AxisValue :type Float%20%28single-precision%29))
  ;[1 1 1] Events
  ;[1 1 1] Handle Player Input
  (bind _canmove (CallFunction|CanMoveinDirection AxisValue))
  (if _canmove
    (Pawn|Input|AddMovementInput "1.000000, 0, 0" AxisValue false)))

(event Input|AxisEvents|InputAxisMove
  (params (AxisValue :type Float%20%28single-precision%29))
  ;[1 1 1] Events
  (Variables|Input|SetRightAmount (* AxisValue (Variables|Input|GetMoveSpeed))))

(fn ConstructionScript)

(fn GetRayBoxCorners
  (params (CornerSelector :type BoxExtentSelector%20Enum))
  (bind _raybox (Variables|Default|GetRayBox))
  (bind (_origin _boxextent) (Collision|GetComponentBounds _raybox))
  (bind (_x _y _z) (Math|Vector|BreakVector _boxextent))
  (Utilities|FlowControl|Sequence
    (:then_0
      (switch Utilities|FlowControl|Switch|SwitchonBoxExtentSelector CornerSelector
        (:NewEnumerator0
          (LocalVariables|SetCornerMod 1.0))
        (:NewEnumerator1
          (LocalVariables|SetCornerMod -1.0))))
    (:then_1
      (return (+ _origin (Math|Vector|MakeVector (* _x (LocalVariables|GetCornerMod)) 0.0 (* _z -1.0)))))))

(fn CanMoveinDirection
  (params (Direction :type Float%20%28single-precision%29))
  ;[1 1 1] Never move on 0.0
  (if (!= Direction 0.0)
    ;[1 1 1] Can move, so set local variable StartOfRay
    (Utilities|FlowControl|Sequence
      (:then_0
        (if (> Direction 0.0)
          (LocalVariables|SetStartOfRay "0, 0, 0")
          (else
            (LocalVariables|SetStartOfRay "0, 0, 0"))))
      (:then_1
        ;[1 1 1] Use StartOfRay and check direction and determine if the object is about to fall off a ledge (can't move)
        (bind _outhit (Collision|LineTraceByChannel (LocalVariables|GetStartOfRay) (+ (LocalVariables|GetStartOfRay) (Math|Vector|MakeVector 0.0 0.0 (* (Variables|RayBoxInfo|GetRayBoxRayLength) -1.0))) "TraceTypeQuery1" false 0 "ForOneFrame"))
        (return (< (.Time (Collision|BreakHitResult _outhit)) 0.4))))
    (else
      (return false))))

(fn UpdatePhysics
  (params (DeltaTime :type Float%20%28single-precision%29) (rayCastResults :type Array%20of%20Ray%20Bundle%20Results%20Structures) (inRayBundle :type Ray%20Bundle%20Results%20Structure))
  (bind _gravityvector (Variables|Physics|GetGravityVector))
  (bind (_x _y _z) (Math|Vector|BreakVector _gravityvector))
  (bind _returnvalue (* _z -1.0))
  (bind _returnvalue_2 (Math|Vector|MakeVector _returnvalue 0.0 _x))
  (bind _returnvalue_3 (Math|Vector|Normalize _returnvalue_2))
  (Utilities|FlowControl|Sequence
    (:then_0
      (LocalVariables|SetPerpGravDir _returnvalue_3)
      ;[1 1 1] Update Velocity
      (Variables|Physics|SetVelocity (+ (* (* _returnvalue_3 (Variables|Input|GetRightAmount)) DeltaTime) (* (Variables|Physics|GetGravityVector) DeltaTime) (Variables|Physics|GetVelocity))))
    (:then_1
      ;[1 1 1] get dV and dP in gravity direction
      (bind (_dposition _dvelocity _washit) (CallFunction|GetDvDpinDirection (Variables|Physics|GetGravityVector) rayCastResults (Variables|Physics|GetVelocity) DeltaTime))
      (LocalVariables|SetDp (+ (LocalVariables|GetDp) _dposition))
      (LocalVariables|SetDv (+ (LocalVariables|GetDv) _dvelocity))
      (if _washit
        _))
    (:then_2
      ;[1 1 1] Get dV dP in right/left direction
      (bind (_dposition_2 _dvelocity_2) (CallFunction|GetDvDpinDirection (LocalVariables|GetPerpGravDir) rayCastResults (Variables|Physics|GetVelocity) DeltaTime))
      (LocalVariables|SetDp (+ (LocalVariables|GetDp) _dposition_2))
      (bind _output_get (LocalVariables|SetDv (+ (LocalVariables|GetDv) _dvelocity_2)))
      (if (> (Math|Vector|VectorLength _output_get) 0.0)
        (Development|PrintString "Hello")))
    (:then_3
      ;[1 1 1] Update velocity and location after collisions
      (Variables|Physics|SetVelocity (+ (LocalVariables|GetDv) (Variables|Physics|GetVelocity)))
      (Transformation|AddActorWorldOffset (LocalVariables|GetDp)))))

(fn CanFall)

(fn GetBoxDirIndexGivenVector
  (params (InVec :type Vector))
  (bind (_x _y _z) (Math|Vector|BreakVector InVec))
  (if (< _z 0.0)
    (return 0 1)
    (elif (> _x 0.0)
      (return 1 2)
      (elif (> _z 0.0)
        (return 2 3)
        (elif (< _x 0.0)
          (return 3 0))))))

(fn HandleVelocityFunc
  (params (Velocity :type Vector) (DirVec :type Vector) (RayCastResults :type Array%20of%20Ray%20Bundle%20Results%20Structures))
  (Utilities|FlowControl|Sequence
    (:then_0
      (bind _outvecindirection (CallFunction|GetVecinDirection Velocity DirVec))
      (bind _output_get (LocalVariables|SetVecInDir _outvecindirection))
      (bind (_index0 _index1) (CallFunction|GetBoxDirIndexGivenVector _output_get))
      (LocalVariables|SetRayBoxIndexValues0 _index0)
      (LocalVariables|SetRayBoxIndexValues1 _index1))
    (:then_1
      ;[1 1 1] Get the minimum ray hit distance (i.e. distance to closest hit point) in gravity direction, and check if we will hit.
      (for (_array_element _array_index) (.WasHit (Utilities|Struct|BreakRayBundleResults (Utilities|Array|Get(acopy) RayCastResults (LocalVariables|GetRayBoxIndexValues0))))
        (if _array_element
          (bind _output_get_2 (LocalVariables|SetMinRayHitDistance (Math|Float|Min(Float) (Utilities|Array|Get(acopy) (.RayHitLengths (Utilities|Struct|BreakRayBundleResults (Utilities|Array|Get(acopy) RayCastResults (LocalVariables|GetRayBoxIndexValues0)))) _array_index) (LocalVariables|GetMinRayHitDistance))))
          (if (<= (Math|Float|Square _output_get_2) (Math|Vector|VectorLengthSquared (LocalVariables|GetVecInDir)))
            (LocalVariables|SetWasHit true)))))
    (:then_2
      (if (LocalVariables|GetWasHit)
        ;[1 1 1] Was hit, so scale the normalized Dir Vec by the hit amount and return that
        (return (* (Math|Vector|Normalize DirVec) (LocalVariables|GetMinRayHitDistance)) true)
        (else
          ;[1 1 1] No hit, just return the input vector amount in dir ection
          (return (LocalVariables|GetVecInDir) false))))))

(fn GetVecinDirection
  (params (InVec :type Vector) (Direction :type Vector))
  (bind _returnvalue (Math|Vector|Normalize Direction))
  (return (* _returnvalue (Math|Vector|DotProduct InVec _returnvalue))))

(fn GetDvDpinDirection
  (params (Direction :type Vector) (InputPin :type Array%20of%20Ray%20Bundle%20Results%20Structures) (Velocity :type Vector) (dT :type Float%20%28single-precision%29))
  (bind _outvecindirection (CallFunction|GetVecinDirection Velocity Direction))
  ;[1 1 1] Handle velocity in gravity direction, and if collision, cancel out velocity in gravity direction.
  (bind _output_get (LocalVariables|SetvelInDir _outvecindirection))
  (bind _output_get_2 (LocalVariables|SetdP (* _output_get dT)))
  (bind (_ouvelindir _encounteredhit) (CallFunction|HandleVelocityFunc _output_get_2 Direction InputPin))
  (if _encounteredhit
    (return _ouvelindir (* (LocalVariables|GetvelInDir) -1.0) true)
    (else
      (return (LocalVariables|GetdP) "0, 0, 0" false))))