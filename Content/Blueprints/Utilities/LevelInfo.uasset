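; LevelInfo is a per-level manager for a 2D Paper tilemap game with rotating gravity.
; On BeginPlay it finds the camera, GraviPlayer and tilemap, links itself to the player, then centers and sizes the orthographic camera from the tilemap bounds.
; RotateLevel steps the camera pitch by 90 degrees in either direction.
; Only down-right rotation also turns the player's gravity vector; down-left leaves it unchanged.
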(event Custom|DoRotateLevel
  (params (RotateEnum :type LevelRotationEnum%20Enum))
  (CallFunction|RotateLevel RotateEnum))

(event EventBeginPlay
  (Utilities|FlowControl|Sequence
    (:then_0
      ;[1 1 1] Sets the current camera to the level's camera
      (bind _outactors (Actor|GetAllActorsOfClass "/Game/Blueprints/Cameras/MyCamera.MyCamera_C"))
      (Variables|GlobalActorRefs|SetLevelCamera (Utilities|Array|Get(acopy) _outactors)))
    (:then_1
      ;[1 1 1] Set up the player references
      (bind _outactors_2 (Actor|GetAllActorsOfClass "/Game/Blueprints/Player/GraviPlayer.GraviPlayer_C"))
      (Variables|/Game/Blueprints/Player/GraviPlayer.GraviPlayer_C|SetLevelInfoRef (Utilities|Array|Get(acopy) _outactors_2) self)
      (Variables|GlobalActorRefs|SetPlayerRef (Utilities|Array|Get(acopy) _outactors_2)))
    (:then_2
      ;[1 1 1] Set up the tilemap reference
      (bind _outactors_3 (Actor|GetAllActorsOfClass "/Script/Paper2D.PaperTileMapActor"))
      (if (> (Utilities|Array|Length _outactors_3) 0)
        (bind _output_get (Variables|Default|SetTileMapRef (Utilities|Array|Get(acopy) _outactors_3)))
        ;[1 1 1] Set the center of the camera to the center of the tile map
        (Utilities|IsValid (Variables|GlobalActorRefs|GetLevelCamera)
          (:Is%20Valid
            (Transformation|SetActorLocation (Variables|GlobalActorRefs|GetLevelCamera) (Math|Vector|MakeVector (.X (Math|Vector|BreakVector (.Origin (Collision|GetComponentBounds (Variables|/Script/Paper2D.PaperTileMapActor|GetRenderComponent _output_get))))) (Variables|Default|GetCameraDepth) (.Z (Math|Vector|BreakVector (.Origin (Collision|GetComponentBounds (Variables|/Script/Paper2D.PaperTileMapActor|GetRenderComponent _output_get)))))) false false)
            ;[1 1 1] Set the camera's ortho
            (Class|CameraComponent|SetOrthoWidth (Variables|/Script/Engine.CameraActor|GetCameraComponent (Variables|GlobalActorRefs|GetLevelCamera)) (+ (Math|Conversions|ToFloat(Integer) (* (Variables|/Game/Blueprints/Cameras/MyCamera.MyCamera_C|GetOrthoPadding (Variables|GlobalActorRefs|GetLevelCamera)) 2)) (.Z (Math|Vector|BreakVector (* (.BoxExtent (Collision|GetComponentBounds (Variables|/Script/Paper2D.PaperTileMapActor|GetRenderComponent _output_get))) 2.0)))))))))))

(event Collision|EventActorBeginOverlap
  (params (OtherActor :type Actor%20Object%20Reference)))

(event EventTick
  (params (DeltaSeconds :type Float%20%28single-precision%29)))

(fn ConstructionScript)

(fn RotateLevel
  (params (RotationDir :type LevelRotationEnum%20Enum))
  (bind _playerref (Variables|GlobalActorRefs|GetPlayerRef))
  (Utilities|FlowControl|Sequence
    (:then_0
      ;[1 1 1] SetCurrentRotation based on rotation input enum
      (switch Utilities|FlowControl|Switch|SwitchonLevelRotationEnum RotationDir
        (:NewEnumerator0
          (bind _output_get (Variables|RotationInfo|SetCurrentRotation (+ (Variables|RotationInfo|GetCurrentRotation) 90)))
          (if (>= _output_get 360)
            (Variables|RotationInfo|SetCurrentRotation 0)))
        (:NewEnumerator1
          (bind _output_get_2 (Variables|RotationInfo|SetCurrentRotation (+ (Variables|RotationInfo|GetCurrentRotation) -90)))
          (if (<= _output_get_2 0)
            (Variables|RotationInfo|SetCurrentRotation 0)))))
    (:then_1
      ;[1 1 1] rotate the camera
      (Transformation|SetActorRotation (Variables|GlobalActorRefs|GetLevelCamera) (Math|Rotator|MakeRotator 0.0 (Math|Conversions|ToFloat(Integer) (Variables|RotationInfo|GetCurrentRotation)) 0.0)))
    (:then_2
      ;[1 1 1] Set the gravity vector with the rotation
      (switch Utilities|FlowControl|Switch|SwitchonLevelRotationEnum RotationDir
        (:NewEnumerator0
          (Variables|/Game/Blueprints/Player/GraviPlayer.GraviPlayer_C|SetBeginGravityVector _playerref (Math|Vector|MakeVector (* (.Z (Math|Vector|BreakVector (Variables|/Game/Blueprints/Player/GraviPlayer.GraviPlayer_C|GetBeginGravityVector _playerref))) -1.0) 0.0 (.X (Math|Vector|BreakVector (Variables|/Game/Blueprints/Player/GraviPlayer.GraviPlayer_C|GetBeginGravityVector _playerref))))))))))