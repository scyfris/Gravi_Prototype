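; Player controller for GraviPlayer that sets the view to MyCamera and routes touch input to either the player or the level tile map.
; Touches on GraviPlayer are forwarded to its press, move and release handlers.
; Dragging the tile map rotates the LevelCamera by the signed angle (atan2 of determinant and dot) around the map's screen-projected center.
; On release, the camera rotation snaps to quarter turns.
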(event EventBeginPlay
  (Variables|/Script/Engine.PlayerController|SetbEnableClickEvents (Game|GetPlayerController 0) true)
  (Variables|Default|SetbEnableMouseOverEvents true)
  (bind _outactors (Actor|GetAllActorsOfClass "/Game/Blueprints/Cameras/MyCamera.MyCamera_C"))
  (Game|Player|SetViewTargetwithBlend (Game|GetPlayerController 0) (Utilities|Array|Get(acopy) _outactors) 0.0 "VTBlend_Linear" 0.0 false)
  ;[1 1 1] Set GraviPlayer variable
  (bind _asgravi_player (Utilities|Casting|CastToGraviPlayer (Game|GetPlayerCharacter 0)))
  (Variables|Default|SetGraviPlayer _asgravi_player)
  ;[1 1 1] Set the level info from the game mode
  (bind _asmy_game_mode (Utilities|Casting|CastToMyGameMode (Game|GetGameMode))
    (:then
      (Variables|Default|SetGameMode _asmy_game_mode))
    (:CastFailed
      (Development|PrintString "FAILED TO GET MY GAME MODE!!"))))

(event EventTick
  (params (DeltaSeconds :type Float%20%28single-precision%29)))

(event Input|TouchEvents|InputTouch
  (params (Location :type Vector) (FingerIndex :type ETouchIndex%20Enum))
  (bind _returnvalue (Game|GetPlayerController 0))
  (bind _returnvalue_2 (Game|GetPlayerController 0))
  (bind (_x _y) (Math|Vector|BreakVector Location))
  (bind _gamemode (Variables|Default|GetGameMode))
  (bind _graviplayer (Variables|Default|GetGraviPlayer))
  (bind _hitresult (Class|PlayerController|GetHitResultUnderFingerbyChannel _returnvalue "Touch1" "TraceTypeQuery1" true))
  (bind _returnvalue_3 (Math|Vector2D|MakeVector2D _x _y))
  (bind _isplayerdragging (Variables|/Game/Blueprints/Player/GraviPlayer.GraviPlayer_C|GetisPlayerDragging _graviplayer))
  (bind _levelinfo (Variables|/Game/Blueprints/Utilities/MyGameMode.MyGameMode_C|GetLevelInfo _gamemode))
  (bind _hitactor (Collision|BreakHitResult _hitresult))
  (bind _tilemapref (Variables|/Game/Blueprints/Utilities/LevelInfo.LevelInfo_C|GetTileMapRef _levelinfo))
  (bind _rendercomponent (Variables|/Script/Paper2D.PaperTileMapActor|GetRenderComponent _tilemapref))
  (bind _origin (Collision|GetComponentBounds _rendercomponent))
  (bind _screenposition (Class|GameplayStatics|ProjectWorldtoScreen _returnvalue_2 _origin false))
  (bind _returnvalue_4 (- _returnvalue_3 _screenposition))
  (bind _returnvalue_5 (Math|Vector2D|Normalize2D _returnvalue_4))
  (bind (_x_2 _y_2) (Math|Vector2D|BreakVector2D _returnvalue_5))
  (:Pressed
    ;[1 1 1] Handle tile map touch events
    (bind _aspaper_tile_map_actor (Utilities|Casting|CastToPaperTileMapActor _hitactor)
      (:then
        (if (== _aspaper_tile_map_actor _tilemapref)
          (Variables|RotationControls|SetTileMapIsDragging true)
          (Variables|RotationControls|SetrcStartTouchPos _returnvalue_3)))
      (:CastFailed
        ;[1 1 1] Handle player touch events
        (bind _asgravi_player (Utilities|Casting|CastToGraviPlayer _hitactor))
        (Default|GraviTouchPressed _asgravi_player))))
  (:Released
    (if _isplayerdragging
      (Default|GraviTouchReleased _asgravi_player)
      (elif (Variables|RotationControls|GetTileMapIsDragging)
        (Variables|RotationControls|SetTileMapIsDragging false)
        ;[1 1 1] Quantize the angle to one of -180, -90, 0, 90, 180
        (bind _output_get (Variables|RotationControls|SetrcOffsetRotation (Math|Conversions|ToFloat(Integer) (Math|Integer|Clamp(Integer) (- (* (Class|KismetSystemLibrary|MakeLiteralInteger (Math|Float|Truncate (/ (+ (Variables|RotationControls|GetrcLastRotation) 225.0) 9e+01))) 90) 180) -180 180))))
        (Transformation|SetActorRotation (Variables|/Game/Blueprints/Utilities/LevelInfo.LevelInfo_C|GetLevelCamera (Variables|/Game/Blueprints/Utilities/MyGameMode.MyGameMode_C|GetLevelInfo (Variables|Default|GetGameMode))) (Math|Rotator|MakeRotator 0.0 _output_get 0.0)))))
  (:Moved
    (if _isplayerdragging
      (Default|GraviTouchMoved _asgravi_player Location)
      (elif (Variables|RotationControls|GetTileMapIsDragging)
        (Development|PrintString (Utilities|String|ToString(Float) (Variables|RotationControls|GetrcOffsetRotation)) true true "(R=0.000000,G=1.000000,B=0.161131,A=1.000000)")
        ;[1 1 1] rotate the camera
        (Transformation|SetActorRotation (Variables|/Game/Blueprints/Utilities/LevelInfo.LevelInfo_C|GetLevelCamera (Variables|/Game/Blueprints/Utilities/MyGameMode.MyGameMode_C|GetLevelInfo (Variables|Default|GetGameMode))) (Math|Rotator|MakeRotator 0.0 (+ (* (Class|KismetMathLibrary|DegAtan2 (- (* _x_2 (.Y (Math|Vector2D|BreakVector2D (Math|Vector2D|Normalize2D (- (Variables|RotationControls|GetrcStartTouchPos) _screenposition))))) (* _y_2 (.X (Math|Vector2D|BreakVector2D (Math|Vector2D|Normalize2D (- (Variables|RotationControls|GetrcStartTouchPos) _screenposition)))))) (Math|Vector2D|DotProduct(2D) _returnvalue_5 (Math|Vector2D|Normalize2D (- (Variables|RotationControls|GetrcStartTouchPos) _screenposition)))) -1.0) (Variables|RotationControls|GetrcOffsetRotation)) 0.0))
        (Variables|RotationControls|SetrcLastRotation (+ (* (Class|KismetMathLibrary|DegAtan2 (- (* _x_2 (.Y (Math|Vector2D|BreakVector2D (Math|Vector2D|Normalize2D (- (Variables|RotationControls|GetrcStartTouchPos) _screenposition))))) (* _y_2 (.X (Math|Vector2D|BreakVector2D (Math|Vector2D|Normalize2D (- (Variables|RotationControls|GetrcStartTouchPos) _screenposition)))))) (Math|Vector2D|DotProduct(2D) _returnvalue_5 (Math|Vector2D|Normalize2D (- (Variables|RotationControls|GetrcStartTouchPos) _screenposition)))) -1.0) (Variables|RotationControls|GetrcOffsetRotation)))))))

(fn ConstructionScript)