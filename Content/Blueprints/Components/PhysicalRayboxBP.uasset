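; Custom 2D physics component that computes movement and collisions from rays cast along the sides of a box, under changeable gravity.
; DoTick casts the rays, integrates gravity and input, then resolves velocity separately along gravity and its perpendicular, applying speed caps, bounciness, ledge checks and constraints.
; It broadcasts velocity, position delta and ray hits through dispatchers, and changes gravity direction on GraviPlayerController's event.
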(event Custom|PlayerCollision
  (params (collisionRayHit :type Hit%20Result%20Structure))
  ;[1 1 1] Use my struct reference, and add 100 to the "myTest" value
  (Default|CallCollisionEventDispatcher collisionRayHit))

(event Custom|ChangeGravity
  (params (newGravityDir :type Vector%202D%20Structure))
  (Variables|MustSetOnce|SetGravity (* newGravityDir (Math|Vector2D|Vector2DLength (Variables|MustSetOnce|GetGravity)))))

(event Custom|CancelTangVelocity
  (if (== (.X (Math|Vector2D|BreakVector2D (Variables|MustSetOnce|GetGravity))) 0.0)
    (Variables|PhysicalProperties|SetCurrentVelocity (Math|Vector2D|MakeVector2D 0.0 (.Y (Math|Vector2D|BreakVector2D (Variables|PhysicalProperties|GetCurrentVelocity)))))
    (else
      (Variables|PhysicalProperties|SetCurrentVelocity (Math|Vector2D|MakeVector2D (.X (Math|Vector2D|BreakVector2D (Variables|PhysicalProperties|GetCurrentVelocity))) 0.0)))))

(event Custom|DoTick
  (params (deltaTime :type Float%20%28single-precision%29))
  (if (not (Variables|PhysicsParameters|GetisPaused))
    (bind (_newvelocity _deltaposition) (CallFunction|UpdatePhysics deltaTime))
    (CallFunction|BroadcastPhysicsUpdate _newvelocity _deltaposition)))

(event Custom|BroadcastPhysicsUpdate
  (params (newVelocity :type Vector%202D%20Structure) (deltaPosition :type Vector%202D%20Structure))
  (Default|CallPhysicsUpdateDispatcher newVelocity deltaPosition))

(event EventBeginPlay
  (bind _asgravi_player_controller (Utilities|Casting|CastToGraviPlayerController (Game|GetPlayerController 0)))
  (EventDispatchers|BindEventtoChangeGravityDirectionDispatcher _asgravi_player_controller (delegate Custom|ChangeGravity)))

(event EventTick
  (params (DeltaSeconds :type Float%20%28single-precision%29)))

(fn UpdatePhysics
  (params (deltaTime :type Float%20%28single-precision%29))
  (Utilities|FlowControl|Sequence
    (:then_0
      (bind _outarraybundles (CallFunction|CasttheRays))
      (bind (_newvelocity _deltaposition _collisionrayhitresults) (CallFunction|UpdateVelocity deltaTime _outarraybundles))
      (for _array_element _collisionrayhitresults
        (CallFunction|PlayerCollision _array_element))
      (return _newvelocity _deltaposition))))

(fn CasttheRays
  (bind _rayboxgeo (Variables|MustSet|GetRayBoxGeo))
  (bind (_origin _boxextent) (Collision|GetComponentBounds _rayboxgeo))
  (Class|RayBox|SetBounds _origin _boxextent)
  (bind _outcorners (Class|RayBox|GetBoxWorldCorners (Math|Vector2D|MakeVector2D 0.0 -1.0)))
  (bind _outrays (Class|RayBox|CastRays (Variables|MustSet|GetRayBoxRayLengths) (Variables|MustSet|GetRayBoxRayOffsets) (Variables|MustSet|GetRayBoxNumRaysPerSide) (Variables|Default|GetDrawDebugLines) 0.0 0.7))
  (return _outrays (Class|GraviUtilities|Convert2DVecArrayto3D _outcorners (.Y (Math|Vector|BreakVector _origin)))))

(fn UpdateVelocity
  (params (deltaTime :type Float%20%28single-precision%29) (rayCastResults :type Array%20of%20Ray%20Bundle%20Structures))
  (bind (_perpgravitydir _perpgravitydirnorm) (CallFunction|GetPerpGravityDirectionNormalized))
  (bind _constraintovector (Variables|Constrains|GetConstrainToVector))
  (bind _rayboxgeo (Variables|MustSet|GetRayBoxGeo))
  (bind _constraintovectorcenter (Variables|Constrains|GetConstrainToVectorCenter))
  (bind _gravity (Variables|MustSetOnce|GetGravity))
  (bind _returnvalue (Transformation|GetWorldLocation _rayboxgeo))
  (bind (_x _y) (Math|Vector2D|BreakVector2D _constraintovector))
  (bind _returnvalue_2 (Class|GraviUtilities|Get2DVector _returnvalue))
  (bind _returnvalue_3 (- _returnvalue_2 _constraintovectorcenter))
  (bind _returnvalue_4 (Math|Vector2D|Vector2DLength _returnvalue_3))
  (Utilities|FlowControl|Sequence
    (:then_0
      (LocalVariables|SetperpGravityDir _perpgravitydir)
      (Variables|PhysicalProperties|SetCurrentVelocity (+ (* (* _perpgravitydirnorm (Variables|MustSet|GetInputForcePerpDir)) deltaTime) (* (Variables|MustSetOnce|GetGravity) deltaTime) (Variables|PhysicalProperties|GetCurrentVelocity))))
    (:then_1
      (if (< (Math|Vector2D|DotProduct(2D) (Variables|PhysicalProperties|GetCurrentVelocity) (LocalVariables|GetperpGravityDir)) 0.0)
        (LocalVariables|SetisMovingLeft true)
        (elif (> (Math|Vector2D|DotProduct(2D) (Variables|PhysicalProperties|GetCurrentVelocity) (LocalVariables|GetperpGravityDir)) 0.0)
          (LocalVariables|SetisMovingRight true))))
    (:then_2
      (bind (_dposition _dvelocity _washit _collisionresultlist _collisionresultrayboxsideindex _collisionresultrayboxsideindexes) (CallFunction|GetDvDpinDirection _gravity rayCastResults deltaTime (or (and (== (Math|Vector2D|DotProduct(2D) _gravity _constraintovector) 0.0) (or (!= _x 0.0) (!= _y 0.0))) (and (and (!= (Variables|Constrains|GetConstrainToVectorLength) 0.0) (>= _returnvalue_4 (Variables|Constrains|GetConstrainToVectorLength))) (not (< (Math|Vector2D|Vector2DLength (- (+ _returnvalue_2 (* (Variables|MustSetOnce|GetGravity) deltaTime)) _constraintovectorcenter)) _returnvalue_4)))) (Variables|MustSet|GetMaxFallSpeed)))
      (LocalVariables|SetdP (+ (LocalVariables|GetdP) _dposition))
      (LocalVariables|SetdV (+ (LocalVariables|GetdV) _dvelocity))
      (if _washit
        (for (_array_element _array_index) _collisionresultlist
          (Utilities|Array|Add (LocalVariables|GetcollisionResults) _array_element)
          (Utilities|Array|Add (LocalVariables|GetcollisionResultsBoxSide) _collisionresultrayboxsideindex)
          (Utilities|Array|Add (LocalVariables|GetcollisionResultsBoxSideHitsIndex) (Utilities|Array|Get(acopy) _collisionresultrayboxsideindexes _array_index)))
        (if (<= (Utilities|Array|Length (LocalVariables|GetcollisionResults)) (/ (Variables|MustSet|GetRayBoxNumRaysPerSide) 2))
          ;[1 1 1] On Ledge! This really needs to be an event back to the player
          (if (== (Utilities|Array|Get(acopy) (LocalVariables|GetcollisionResultsBoxSideHitsIndex)) 0)
            (LocalVariables|SetcanMoveRight false)
            (else
              (LocalVariables|SetcanMoveLeft false))))))
    (:then_3
      (bind (_dposition_2 _dvelocity_2 _washit_2 _collisionresultlist_2) (CallFunction|GetDvDpinDirection (LocalVariables|GetperpGravityDir) rayCastResults deltaTime (or (or (or (and (not (LocalVariables|GetcanMoveRight)) (LocalVariables|GetisMovingRight)) (and (not (LocalVariables|GetcanMoveLeft)) (LocalVariables|GetisMovingLeft))) (LocalVariables|GetshouldHaltFromInputTouch)) (Variables|Constrains|GetConstrainToGravity)) (Variables|MustSet|GetMaxMovespeed)))
      (bind _output_get (LocalVariables|SetdpTang _dposition_2))
      (LocalVariables|SetdP (+ (LocalVariables|GetdP) _output_get))
      (bind _output_get_2 (LocalVariables|SetdV (+ _dvelocity_2 (LocalVariables|GetdV))))
      (if (> (Math|Vector2D|Vector2DLength _output_get_2) 0.0)
        (for _array_element_2 _collisionresultlist_2
          (Utilities|Array|Add (LocalVariables|GetcollisionResults) _array_element_2))))
    (:then_4
      (Variables|PhysicalProperties|SetCurrentVelocity (+ (LocalVariables|GetdV) (Variables|PhysicalProperties|GetCurrentVelocity)))
      (return (Variables|PhysicalProperties|GetCurrentVelocity) (LocalVariables|GetdP) (LocalVariables|GetcollisionResults)))))

(fn GetDvDpinDirection
  (params (Direction :type Vector%202D%20Structure) (RayBundleResults :type Array%20of%20Ray%20Bundle%20Structures) (dT :type Float%20%28single-precision%29) (CancelVelocity :type Boolean) (MaxVelInDir :type Float%20%28single-precision%29))
  (bind _currentvelocity (Variables|PhysicalProperties|GetCurrentVelocity))
  (bind _outvec (Class|GraviUtilities|GetVectorinDirection _currentvelocity Direction))
  (bind _returnvalue (Math|Vector2D|Vector2DLength _outvec))
  (Utilities|FlowControl|Sequence
    (:then_0
      (if (> _returnvalue MaxVelInDir)
        (LocalVariables|SetvelInDir (* (/ _outvec _returnvalue) MaxVelInDir))
        (else
          (LocalVariables|SetvelInDir _outvec))))
    (:then_1
      (if CancelVelocity
        ;[1 1 1] Input says we shuld just cancel out velocity
        (return "" (* (LocalVariables|GetvelInDir) -1.0) false (Utilities|Array|MakeArray "") 0 (Utilities|Array|MakeArray 0))
        (else
          (bind _output_get (LocalVariables|SetdP (* (LocalVariables|GetvelInDir) dT)))
          (bind (_outvelindir _encounteredhit _collisionresultlist _collisionresultrayboxsideindexes _collisionresultrayboxsideindex) (CallFunction|HandleVelocityFunc _output_get Direction RayBundleResults))
          (if _encounteredhit
            (return _outvelindir (* (LocalVariables|GetvelInDir) (- -1.0 (Variables|MustSet|GetBounciness))) true _collisionresultlist _collisionresultrayboxsideindex _collisionresultrayboxsideindexes)
            (else
              (return (LocalVariables|GetdP) "" false _collisionresultlist _collisionresultrayboxsideindex _collisionresultrayboxsideindexes))))))))

(fn HandleVelocityFunc
  (params (velocity :type Vector%202D%20Structure) (dirVec :type Vector%202D%20Structure) (rayBundleResults :type Array%20of%20Ray%20Bundle%20Structures))
  (if (== (Class|KismetMathLibrary|VSize2DSquared velocity) 0.0)
    (return "" false (Utilities|Array|MakeArray "") (Utilities|Array|MakeArray 0) 0)
    (else
      (Utilities|FlowControl|Sequence
        (:then_0
          (bind _output_get (LocalVariables|SetvecInDir (Class|GraviUtilities|GetVectorinDirection velocity dirVec)))
          (LocalVariables|SetrayBoxCornerIndex0 (Class|GraviUtilities|GetQuadrantFirstIndex _output_get))
          (LocalVariables|SetrayBoxCornerIndex1 (Math|Integer|%(Integer) (+ (Class|GraviUtilities|GetQuadrantFirstIndex _output_get) 1) 4)))
        (:then_1
          (for (_array_element _array_index) (.WasHit (Utilities|Struct|BreakRayBundle (Utilities|Array|Get(acopy) rayBundleResults (LocalVariables|GetrayBoxCornerIndex0))))
            (if _array_element
              (LocalVariables|SetminRayHitDistance (Math|Float|Min(Float) (Utilities|Array|Get(acopy) (.RayHitLengths (Utilities|Struct|BreakRayBundle (Utilities|Array|Get(acopy) rayBundleResults (LocalVariables|GetrayBoxCornerIndex0)))) _array_index) (LocalVariables|GetminRayHitDistance)))
              (if (<= (Math|Float|Square (Utilities|Array|Get(acopy) (.RayHitLengths (Utilities|Struct|BreakRayBundle (Utilities|Array|Get(acopy) rayBundleResults (LocalVariables|GetrayBoxCornerIndex0)))) _array_index)) (Class|KismetMathLibrary|VSize2DSquared (LocalVariables|GetvecInDir)))
                (LocalVariables|SetwasHit true)
                (Utilities|Array|Add (LocalVariables|GethitResultList) (Utilities|Array|Get(acopy) (.HitResults (Utilities|Struct|BreakRayBundle (Utilities|Array|Get(acopy) rayBundleResults (LocalVariables|GetrayBoxCornerIndex0)))) _array_index))
                (Utilities|Array|Add (LocalVariables|GetHitResultListRayIndexes) _array_index)
                (LocalVariables|SetHitResultRayBoxSideIndex (LocalVariables|GetrayBoxCornerIndex0))))))
        (:then_2
          (if (LocalVariables|GetwasHit)
            (return (* (Math|Vector2D|Normalize2D dirVec) (LocalVariables|GetminRayHitDistance)) true (LocalVariables|GethitResultList) (LocalVariables|GetHitResultListRayIndexes) (LocalVariables|GetHitResultRayBoxSideIndex))
            (else
              (return (LocalVariables|GetvecInDir) false (Utilities|Array|MakeArray "") (Utilities|Array|MakeArray 0) -1))))))))

(fn GetPerpGravityDirectionNormalized
  (bind _gravity (Variables|MustSetOnce|GetGravity))
  (bind _returnvalue (Class|GraviUtilities|GetPerpDirectionCounterClockwise2D _gravity))
  (bind _returnvalue_2 (Math|Vector2D|Vector2DLength _returnvalue))
  (return _returnvalue (/ _returnvalue _returnvalue_2) _returnvalue_2))